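; Game mode for an infinite terrain game that spawns chained tiles and keeps score.
; On BeginPlay it populates a nav mesh bounds volume pool, then spawns a short initial run of BP_Tile actors.
; SpawnTile hands each tile the shared pool and stores its attach location as the next spawn transform, so tiles link end to end.
; NewTileConquered increments the score without spawning further tiles.
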(event EventBeginPlay
  (Class|InfiniteTerrainGameMode|PopulateBoundsVolumePool)
  (for _index (range 0 3)
    (CallFunction|SpawnTile)))

(fn ConstructionScript)

(fn SpawnTile
  (bind _returnvalue (Game|SpawnActorfromClass "/Game/Dynamic/Terrain/BP_Tile.BP_Tile_C" (Variables|Default|GetLastTransform) "Undefined" 0 0))
  (Class|Tile|SetPool _returnvalue (Variables|Default|GetNavMeshBoundsVolumePool))
  (bind _attachtransform (Default|GetAttachLocation _returnvalue))
  (Variables|Default|SetLastTransform _attachtransform))

(fn NewTileConquered
  (Math|Integer|IncrementInt (Variables|Default|GetScore)))