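; Terrain tile for an infinite level that populates itself on BeginPlay with scattered containers, boxes, canisters, scaled rocks and a few AI characters.
; Its barrier starts locked, turning passable and green while the player overlaps the locking volume, then solid and red when they leave.
; When the player enters the deletion volume, it asks InfiniteTerrainGameMode for a new tile and destroys itself.
; GetAttachLocation exposes the AttachPoint transform.
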(event OnComponentBeginOverlap(DeletionVolume)
  (params (OverlappedComponent :type Primitive%20Component%20Object%20Reference) (OtherActor :type Actor%20Object%20Reference) (OtherComp :type Primitive%20Component%20Object%20Reference) (OtherBodyIndex :type Integer) (bFromSweep :type Boolean) (SweepResult :type Hit%20Result%20Structure%20%28by%20ref%29))
  (Utilities|IsPlayerActor OtherActor)
  (CallFunction|SpawnNewTile)
  (Actor|DestroyActor))

(event OnComponentEndOverlap(LockingVolume)
  (params (OverlappedComponent :type Primitive%20Component%20Object%20Reference) (OtherActor :type Actor%20Object%20Reference) (OtherComp :type Primitive%20Component%20Object%20Reference) (OtherBodyIndex :type Integer))
  (Utilities|IsPlayerActor OtherActor)
  (CallFunction|Lock))

(event OnComponentBeginOverlap(LockingVolume)
  (params (OverlappedComponent :type Primitive%20Component%20Object%20Reference) (OtherActor :type Actor%20Object%20Reference) (OtherComp :type Primitive%20Component%20Object%20Reference) (OtherBodyIndex :type Integer) (bFromSweep :type Boolean) (SweepResult :type Hit%20Result%20Structure%20%28by%20ref%29))
  (Utilities|IsPlayerActor OtherActor)
  (CallFunction|Unlock))

(event EventBeginPlay
  (CallFunction|Lock)
  (Class|Tile|PlaceActors "/Game/Dynamic/Terrain/Props/BP_Container.BP_Container_C" (Utilities|Struct|MakeGenerationParameters 1 3 4.5e+02 1.0 1.0))
  (Class|Tile|PlaceActors "/Game/Dynamic/Terrain/Props/BP_Box.BP_Box_C" (Utilities|Struct|MakeGenerationParameters 1 8 1e+02 1.0 1.0))
  (Class|Tile|PlaceActors "/Game/Dynamic/Terrain/Props/BP_Canister.BP_Canister_C" (Utilities|Struct|MakeGenerationParameters 1 9 5e+01 1.0 1.0))
  (Class|Tile|PlaceActors "/Game/Dynamic/Terrain/Props/BP_Rock1.BP_Rock1_C" (Utilities|Struct|MakeGenerationParameters 1 3 1.5e+02 1.0 5.0))
  (Class|Tile|PlaceActors "/Game/Dynamic/Terrain/Props/BP_Rock2.BP_Rock2_C" (Utilities|Struct|MakeGenerationParameters 1 3 2.5e+02 1.0 5.0))
  (Class|Tile|PlaceActors "/Game/Dynamic/Terrain/Props/BP_Rock3.BP_Rock3_C" (Utilities|Struct|MakeGenerationParameters 1 3 2.5e+02 1.0 5.0))
  (Class|Tile|PlaceAIPawns "/Game/Dynamic/Character/Behavior/BP_Character.BP_Character_C" (Utilities|Struct|MakeGenerationParameters 2 4 1e+02 1.0 1.0)))

(fn ConstructionScript)

(fn GetAttachLocation
  (return (Transformation|GetWorldTransform (Variables|Default|GetAttachPoint))))

(fn Unlock
  (bind _barrier (Variables|Default|GetBarrier))
  (Development|PrintString "unlocking")
  (Collision|SetCollisionEnabled _barrier "NoCollision")
  (Rendering|Material|SetMaterial _barrier 0 "/Game/Dynamic/Terrain/M_Barrier_Green.M_Barrier_Green"))

(fn Lock
  (bind _barrier (Variables|Default|GetBarrier))
  (Development|PrintString "locking")
  (Collision|SetCollisionEnabled _barrier "QueryAndPhysics")
  (Rendering|Material|SetMaterial _barrier 0 "/Game/Dynamic/Terrain/M_Barrier_Red.M_Barrier_Red"))

(fn SpawnNewTile
  (bind _asinfinite_terrain_game_mode (Utilities|Casting|CastToInfiniteTerrainGameMode (Game|GetGameMode)))
  (Default|SpawnTile _asinfinite_terrain_game_mode))